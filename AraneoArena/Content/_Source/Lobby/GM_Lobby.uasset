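; Lobby game mode that brings each joining player into the lobby and cleans up when they leave.
; PostLogin shows a loading screen, has GI_AraneoArena load saved user data into the lobby player state, then sets the view and shows the lobby UI.
; Fixed delays pace these steps rather than readiness checks.
; Logout destroys the exiting controller's pawn, and an unreferenced CustomWhile macro provides a delay-based polling loop.
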(event `self.K2_PostLogin`
  (params (NewPlayer :type "PlayerController Object Reference"))
  ;[1 1 1] Show the loading screen, set the view and show the lobby UI, then remove the loading screen
  (bind _aspc_lobby (cast `/Game/_Source/Lobby/PC_Lobby` NewPlayer))
  (`/Game/_Source/Lobby/PC_Lobby.ShowLoadingScreen` _aspc_lobby)
  (`KismetSystemLibrary.Delay` 1.5)
  (bind _asgi_araneo_arena (cast `/Game/_Source/GI_AraneoArena` (`GameplayStatics.GetGameInstance`)))
  (`/Game/_Source/GI_AraneoArena.LoadSavedUserDataAndSetLobbyPS` _asgi_araneo_arena _aspc_lobby)
  (`KismetSystemLibrary.Delay` 1.5)
  (`/Game/_Source/Lobby/PC_Lobby.SetView` _aspc_lobby)
  (`/Game/_Source/Lobby/PC_Lobby.ShowLobbyUI` _aspc_lobby)
  (`/Game/_Source/Lobby/PC_Lobby.RemoveLoadingScreen` _aspc_lobby true "NewEnumerator2"))

(event `self.K2_OnLogout`
  (params (ExitingController :type "Controller Object Reference"))
  ;[1 1 1] On logout, free up spawn point and destroy chosen character
  (`self.K2_DestroyActor` (`Controller.K2_GetPawn` ExitingController)))

(fn `UserConstructionScript`)