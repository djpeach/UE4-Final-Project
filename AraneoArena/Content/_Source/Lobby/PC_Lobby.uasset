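; Lobby player controller that manages the lobby camera, UI screens and the player's username and character choice.
; Implements lobby UI and loading screen interfaces through handler events that lazily create widgets and set cursor and input modes.
; Username changes are written to PS_Lobby, whose value also fills the lobby UI.
; Character changes spawn and possess a replacement pawn, then SetView blends to a spawned lobby camera after a delay.
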(event `self.ReceiveBeginPlay`
  ;[1 1 1] Initialize some references on BeginPlay
  (bind _asps_lobby (cast `/Game/_Source/Lobby/PS_Lobby` (`self.PlayerState`)))
  (set `self.PSRef` _asps_lobby))

(event `SetView`
  (params (Duration :type "Float (double-precision)" :default 1.0))
  ;[1 1 1] Create the lobby camera and set it as the view target
  (`KismetSystemLibrary.Delay` Duration)
  (`/Engine/EditorBlueprintResources/StandardMacros.IsValid` (`self.LobbyCamera`)
    (:`Is Valid`
      _)
    (:`Is Not Valid`
      (bind _returnvalue (`|SpawnActorFromClass` "/Script/Engine.CameraActor" (`KismetMathLibrary.MakeTransform` (75.0 -225.0 250.0) (struct :`Pitch` 0.5)) "AlwaysSpawn" "OverrideRootScale" self null))
      (bind _output_get (set `self.LobbyCamera` _returnvalue))))
  (`self.SetViewTargetWithBlend` _output_get))

(event `ChangeUsername`
  (params (NewUsername :type String))
  (bind _asps_lobby (cast `/Game/_Source/Lobby/PS_Lobby` (`self.PlayerState`)))
  (set `/Game/_Source/Lobby/PS_Lobby.Username` NewUsername _asps_lobby))

(event `ChangeCharacter`
  (params (NewCharacter :type "/Game/_Source/Characters/PlayerCharacters/CharacterSelection/CharacterChoice Structure"))
  (bind _returnvalue (`self.K2_GetPawn`))
  (`self.SetActorHiddenInGame` _returnvalue true)
  (bind _returnvalue_2 (`|SpawnActorFromClass` (`.BPClass_7_78B4B0E84E1A7BF3A4A6C1B589C662F9` (break `/Game/_Source/Characters/PlayerCharacters/CharacterSelection/CharacterChoice` NewCharacter)) (`self.GetTransform` _returnvalue) "AlwaysSpawn" "OverrideRootScale" self null))
  (`self.K2_DestroyActor` _returnvalue)
  (`self.Possess` _returnvalue_2)
  (`self.SetView` 1.5))

(event `Handler_ShowLobbyUI`
  ;[1 1 1] Show the lobby UI
  (`/Engine/EditorBlueprintResources/StandardMacros.IsValid` (`self.LobbyUI`)
    (:`Is Valid`
      _)
    (:`Is Not Valid`
      (bind _returnvalue (`|CreateWidget` "/Game/_Source/Lobby/UI/LobbyUI.LobbyUI_C" self))
      (bind _output_get (set `self.LobbyUI` _returnvalue))))
  (bind _asps_lobby (cast `/Game/_Source/Lobby/PS_Lobby` (`self.PlayerState`)))
  (`EditableTextBox.SetText` (`/Game/_Source/Lobby/UI/LobbyUI.UsernameInput` _output_get) (`KismetTextLibrary.Conv_StringToText` (`/Game/_Source/Lobby/PS_Lobby.Username` _asps_lobby)))
  (`UserWidget.AddToViewport` _output_get 0)
  (set `self.bShowMouseCursor` true)
  (`WidgetBlueprintLibrary.SetInputMode_GameAndUIEx` self null))

(event `/Game/_Source/Lobby/INT_LobbyUIManager.ShowLobbyUI`
  ;[1 1 1] Show the lobby UI
  (`self.Handler_ShowLobbyUI`))

(event `Handler_ShowCharacterSelect`
  ;[1 1 1] Show the character select screen
  (if (`KismetSystemLibrary.IsValid` (`self.CharacterSelectUI`))
    (`Widget.SetVisibility` (`self.CharacterSelectUI`) "Visible")
    (else
      (bind _returnvalue (`|CreateWidget` "/Game/_Source/Lobby/UI/CharacterSelect.CharacterSelect_C" self))
      (bind _output_get (set `self.CharacterSelectUI` _returnvalue))
      (`UserWidget.AddToViewport` _output_get 0)))
  (set `self.bShowMouseCursor` true)
  (`WidgetBlueprintLibrary.SetInputMode_UIOnlyEx` self (`self.CharacterSelectUI`)))

(event `/Game/_Source/Lobby/INT_LobbyUIManager.ShowCharacterSelect`
  ;[1 1 1] Show the character select screen
  (`self.Handler_ShowCharacterSelect`))

(event `Handler_HideCharacterSelect`
  ;[1 1 1] Remove the character select screen
  (bind _characterselectui (`self.CharacterSelectUI`)
    (:`then`
      (`Widget.SetVisibility` _characterselectui "Hidden")
      (`WidgetBlueprintLibrary.SetInputMode_GameAndUIEx` self (`self.LobbyUI`)))
    (:`else`)))

(event `/Game/_Source/Lobby/INT_LobbyUIManager.HideCharacterSelect`
  ;[1 1 1] Remove the character select screen
  (`self.Handler_HideCharacterSelect`))

(event `Handler_ShowLoadingScreen`
  ;[1 1 1] Show the loading screen, blocking the entire screen
  (`self.LoadingScreen`
    (:`then`
      _)
    (:`else`
      (bind _returnvalue (`|CreateWidget` "/Game/_Source/Shared/UI/LoadingScreen.LoadingScreen_C" self))
      (bind _output_get (set `self.LoadingScreen` _returnvalue))))
  (`UserWidget.AddToViewport` _output_get 999)
  (set `self.bShowMouseCursor` false)
  (`WidgetBlueprintLibrary.SetInputMode_UIOnlyEx` self null))

(event `/Game/_Source/Shared/INT_LoadingScreenManager.ShowLoadingScreen`
  ;[1 1 1] Show the loading screen, blocking the entire screen
  (`self.Handler_ShowLoadingScreen`))

(event `Handler_DismissLoadingScreen`
  (params (bShowMouseCursor :type Boolean) (Selection :type "/Game/_Source/Shared/InputMode Enum" :default "NewEnumerator0"))
  ;[1 1 1] Remove the loading screen and reset input mode and mouse cursor appropriately
  (bind _loadingscreen (`self.LoadingScreen`)
    (:`then`
      (`Widget.RemoveFromParent` _loadingscreen)
      (set `self.bShowMouseCursor` bShowMouseCursor)
      (switch `/Game/_Source/Shared/InputMode` Selection
        (:`NewEnumerator0`
          (`WidgetBlueprintLibrary.SetInputMode_UIOnlyEx` self null))
        (:`NewEnumerator1`
          (`WidgetBlueprintLibrary.SetInputMode_GameOnly` self))
        (:`NewEnumerator2`
          (`WidgetBlueprintLibrary.SetInputMode_GameAndUIEx` self null))))
    (:`else`)))

(event `/Game/_Source/Shared/INT_LoadingScreenManager.DismissLoadingScreen`
  (params (bShowMouseCursor :type Boolean) (InputMode :type "/Game/_Source/Shared/InputMode Enum" :default "NewEnumerator0"))
  ;[1 1 1] Remove the loading screen and reset input mode and mouse cursor appropriately
  (`self.Handler_DismissLoadingScreen` bShowMouseCursor InputMode))

(fn `UserConstructionScript`)