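; Player controller for the menu system that opens the main, play, profile, server browser and host config menus.
; Each INT_MenuManager event lazily creates its widget on first call, caches it in a variable and adds it to the viewport.
; It then shows the mouse cursor and switches to UI-only input focused on that menu.
; Nothing here removes previously shown menus, and BeginPlay and Tick are unused.
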(event `/Game/_Source/MenuSystem/INT_MenuManager.ShowMainMenu`
  (`/Engine/EditorBlueprintResources/StandardMacros.IsValid` (`self.MainMenu`)
    (:`Is Valid`
      _)
    (:`Is Not Valid`
      (bind _returnvalue (`|CreateWidget` "/Game/_Source/MenuSystem/UI/MainMenu.MainMenu_C" self))
      (bind _output_get (set `self.MainMenu` _returnvalue))))
  (`UserWidget.AddToViewport` _output_get 0)
  (set `self.bShowMouseCursor` true)
  (`WidgetBlueprintLibrary.SetInputMode_UIOnlyEx` self (`self.MainMenu`)))

(event `/Game/_Source/MenuSystem/INT_MenuManager.ShowPlayMenu`
  (`/Engine/EditorBlueprintResources/StandardMacros.IsValid` (`self.PlayMenu`)
    (:`Is Valid`
      _)
    (:`Is Not Valid`
      (bind _returnvalue (`|CreateWidget` "/Game/_Source/MenuSystem/UI/PlayMenu.PlayMenu_C" self))
      (bind _output_get (set `self.PlayMenu` _returnvalue))))
  (`UserWidget.AddToViewport` _output_get 0)
  (set `self.bShowMouseCursor` true)
  (`WidgetBlueprintLibrary.SetInputMode_UIOnlyEx` self (`self.PlayMenu`)))

(event `/Game/_Source/MenuSystem/INT_MenuManager.ShowProfileMenu`
  (`/Engine/EditorBlueprintResources/StandardMacros.IsValid` (`self.ProfileMenu`)
    (:`Is Valid`
      _)
    (:`Is Not Valid`
      (bind _returnvalue (`|CreateWidget` "/Game/_Source/MenuSystem/UI/ProfileMenu.ProfileMenu_C" self))
      (bind _output_get (set `self.ProfileMenu` _returnvalue))))
  (`UserWidget.AddToViewport` _output_get 0)
  (set `self.bShowMouseCursor` true)
  (`WidgetBlueprintLibrary.SetInputMode_UIOnlyEx` self (`self.ProfileMenu`)))

(event `/Game/_Source/MenuSystem/INT_MenuManager.ShowServerBrowserMenu`
  (`/Engine/EditorBlueprintResources/StandardMacros.IsValid` (`self.ServerBrowserMenu`)
    (:`Is Valid`
      _)
    (:`Is Not Valid`
      (bind _returnvalue (`|CreateWidget` "/Game/_Source/MenuSystem/UI/ServerBrowserMenu.ServerBrowserMenu_C" self))
      (bind _output_get (set `self.ServerBrowserMenu` _returnvalue))))
  (`UserWidget.AddToViewport` _output_get 0)
  (set `self.bShowMouseCursor` true)
  (`WidgetBlueprintLibrary.SetInputMode_UIOnlyEx` self (`self.ServerBrowserMenu`)))

(event `/Game/_Source/MenuSystem/INT_MenuManager.ShowHostConfigMenu`
  (`/Engine/EditorBlueprintResources/StandardMacros.IsValid` (`self.HostConfigMenu`)
    (:`Is Valid`
      _)
    (:`Is Not Valid`
      (bind _returnvalue (`|CreateWidget` "/Game/_Source/MenuSystem/UI/HostConfigMenu.HostConfigMenu_C" self))
      (bind _output_get (set `self.HostConfigMenu` _returnvalue))))
  (`UserWidget.AddToViewport` _output_get 0)
  (set `self.bShowMouseCursor` true)
  (`WidgetBlueprintLibrary.SetInputMode_UIOnlyEx` self (`self.HostConfigMenu`)))

(fn `UserConstructionScript`)