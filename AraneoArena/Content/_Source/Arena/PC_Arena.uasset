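; Player controller for the Arena that manages the loading screen and HUD cleanup and starts in game-only input.
; Loading screen interface events call handlers that lazily create and reuse one widget at top Z-order with UI-only input.
; On dismissal, the caller chooses cursor visibility and input mode.
; HUD clearing routes through a handler event on the server and removes all widgets directly otherwise.
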(event `self.ReceiveBeginPlay`
  (`/Game/_Source/Shared/Utils.Assert` (`self.IsLocalController`))
  (`WidgetBlueprintLibrary.SetInputMode_GameOnly` self))

(event `Handler_ShowLoadingScreen`
  ;[1 1 1] Show the loading screen, blocking the entire screen
  (`self.LoadingScreen`
    (:`then`
      _)
    (:`else`
      (bind _returnvalue (`|CreateWidget` "/Game/_Source/Shared/UI/LoadingScreen.LoadingScreen_C" self))
      (bind _output_get (set `self.LoadingScreen` _returnvalue))))
  (`UserWidget.AddToViewport` _output_get 999)
  (set `self.bShowMouseCursor` false)
  (`WidgetBlueprintLibrary.SetInputMode_UIOnlyEx` self null))

(event `/Game/_Source/Shared/INT_LoadingScreenManager.ShowLoadingScreen`
  ;[1 1 1] Show the loading screen, blocking the entire screen
  (`KismetSystemLibrary.PrintString` "Show Loading screen" true true (struct :`R` 0.06782 :`G` 1.0 :`A` 1.0) 10.0)
  (`self.Handler_ShowLoadingScreen`))

(event `Handler_DismissLoadingScreen`
  (params (bShowMouseCursor :type Boolean) (Selection :type "/Game/_Source/Shared/InputMode Enum" :default "NewEnumerator0"))
  ;[1 1 1] Remove the loading screen and reset input mode and mouse cursor appropriately
  (bind _loadingscreen (`self.LoadingScreen`)
    (:`then`
      (`Widget.RemoveFromParent` _loadingscreen)
      (set `self.bShowMouseCursor` bShowMouseCursor)
      (switch `/Game/_Source/Shared/InputMode` Selection
        (:`NewEnumerator0`
          (`WidgetBlueprintLibrary.SetInputMode_UIOnlyEx` self null))
        (:`NewEnumerator1`
          (`WidgetBlueprintLibrary.SetInputMode_GameOnly` self))
        (:`NewEnumerator2`
          (`WidgetBlueprintLibrary.SetInputMode_GameAndUIEx` self null))))
    (:`else`
      (`KismetSystemLibrary.PrintString` "Loading Screen not valid" true true (struct :`G` 1.0 :`B` 0.003194 :`A` 1.0) 10.0))))

(event `/Game/_Source/Shared/INT_LoadingScreenManager.DismissLoadingScreen`
  (params (bShowMouseCursor :type Boolean) (InputMode :type "/Game/_Source/Shared/InputMode Enum" :default "NewEnumerator0"))
  ;[1 1 1] Remove the loading screen and reset input mode and mouse cursor appropriately
  (`KismetSystemLibrary.PrintString` "Dismiss loading screen" true true (struct :`G` 1.0 :`B` 0.000306 :`A` 1.0) 10.0)
  (`self.Handler_DismissLoadingScreen` bShowMouseCursor InputMode))

(event `HandlerRemoveAllHUDWidgets`
  ;[1 1 1] Remove all widgets from screen
  (`WidgetLayoutLibrary.RemoveAllWidgets`))

(event `/Game/_Source/Arena/INT_ArenaHUDManager.RemoveAllHUDWidgets`
  ;[1 1 1] Remove all widgets from screen
  (if (`KismetSystemLibrary.IsServer`)
    (`self.HandlerRemoveAllHUDWidgets`)
    (else
      (`WidgetLayoutLibrary.RemoveAllWidgets`))))

(fn `UserConstructionScript`)