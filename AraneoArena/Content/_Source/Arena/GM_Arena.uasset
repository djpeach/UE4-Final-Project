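; Arena game mode that brings players into the match after their controller is swapped to PC_Arena and spawns the character class stored in each PS_Arena.
; Arriving controllers get a loading screen and join a queue, which is initialized one player at a time with fixed delays, guarded by a busy flag.
; Each pass links controller to player state, refreshes username headers on all connected players' pawns, then dismisses that player's loading screen.
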(event `self.K2_OnSwapPlayerControllers`
  (params (OldPC :type "PlayerController Object Reference") (NewPC :type "PlayerController Object Reference"))
  ;[1 1 1] When a player gets their pc swapped to the pc_arena, add them to the incoming players queue. Kick off the init function if it is not already running
  (bind _aspc_arena (cast `/Game/_Source/Arena/PC_Arena` NewPC)
    (:`then`
      (`self.Log` "Casted to PC_Arena" :!enabledstate Disabled)
      (message `/Game/_Source/Shared/INT_LoadingScreenManager.ShowLoadingScreen` _aspc_arena)
      (`KismetArrayLibrary.Array_AddUnique` (`self.IncomingPlayers`) _aspc_arena)
      (`self.Log` (`KismetStringLibrary.Concat_StrStr` "Added: " (`KismetSystemLibrary.GetDisplayName` _aspc_arena) " to IncomingPlayers") :!enabledstate Disabled)
      (`/Game/_Source/Shared/Utils.Assert` (not (`self.InitializingPlayer`)))
      (`self.Log` "Initializing Player is false, so kicking off InitializePlayerToArena" :!enabledstate Disabled)
      (`self.InitializePlayerToArena`))
    (:`CastFailed`
      (`self.Log` "Failed casting to PC_Arena" :!enabledstate Disabled))))

(event `InitializePlayerToArena`
  (bind _incomingplayers (`self.IncomingPlayers`))
  (bind _returnvalue (`KismetArrayLibrary.Array_Length` _incomingplayers))
  (bind _output (`|GetArrayItem` (`self.IncomingPlayers`)))
  ;[1 1 1] Init each player in the queue
  (`self.Log` "Initializing" :!enabledstate Disabled)
  (set `self.InitializingPlayer` true)
  (`KismetSystemLibrary.Delay` 1.5)
  (`self.Log` (`KismetStringLibrary.Concat_StrStr` "Got: " (`KismetSystemLibrary.GetDisplayName` _output)) :!enabledstate Disabled)
  (bind _asps_arena (cast `/Game/_Source/Arena/PS_Arena` (`Controller.PlayerState` _output))
    (:`then`
      (`self.Log` "Casted to PS_Arena" :!enabledstate Disabled)
      (set `/Game/_Source/Arena/PS_Arena.PCRef` _output _asps_arena)
      (`KismetSystemLibrary.Delay` 3.0)
      (`self.SetupEachConnectedPlayer`)
      (message `/Game/_Source/Shared/INT_LoadingScreenManager.DismissLoadingScreen` _output false "NewEnumerator1")
      (`KismetArrayLibrary.Array_Remove` _incomingplayers)
      (if (> _returnvalue 0)
        (`self.Log` (`KismetStringLibrary.Concat_StrStr` (`KismetStringLibrary.Conv_IntToString` _returnvalue) " players left to process") :!enabledstate Disabled)
        (`self.InitializePlayerToArena`)
        (else
          (`self.Log` "No players left to process" :!enabledstate Disabled)
          (set `self.InitializingPlayer` false))))
    (:`CastFailed`
      (`self.Log` "Failed casting to PS_Arena" :!enabledstate Disabled))))

(event `SetupEachConnectedPlayer`
  ;[1 1 1] Share data with every other currently connected player, right now just username
  (`self.Log` "Setting up each connected player" :!enabledstate Disabled)
  (bind _asgs_arena (cast `/Game/_Source/Arena/GS_Arena` (`GameplayStatics.GetGameState`))
    (:`then`
      (`self.Log` "Casted to GS_Arena" :!enabledstate Disabled)
      (for _array_element (`GameStateBase.PlayerArray` _asgs_arena)
        (bind _asps_arena (cast `/Game/_Source/Arena/PS_Arena` _array_element)
          (:`then`
            (`self.Log` "Casted to PS_Areana" :!enabledstate Disabled)
            (bind _username (`/Game/_Source/Arena/PS_Arena.Username` _asps_arena))
            (`self.Log` (`KismetStringLibrary.Concat_StrStr` "Setting header for " _username " on all clients") :!enabledstate Disabled)
            (bind _asbp_base_player (cast `/Game/_Source/Characters/PlayerCharacters/BP_BasePlayer` (`Controller.K2_GetPawn` (`/Game/_Source/Arena/PS_Arena.PCRef` _asps_arena)))
              (:`then`
                (`self.Log` "Casted to BP_BasePlayer" :!enabledstate Disabled)
                (`/Game/_Source/Characters/PlayerCharacters/BP_BasePlayer.SetHeaderText` _asbp_base_player _username))
              (:`CastFailed`
                (`self.Log` "Failed casting to BP_BasePlayer" :!enabledstate Disabled))))
          (:`CastFailed`
            (`self.Log` "Failed casting to PS_Areana" :!enabledstate Disabled)))))
    (:`CastFailed`
      (`self.Log` "Failed casting to GS_Arena" :!enabledstate Disabled))))

(fn `GetDefaultPawnClassForController`
  (params (InController :type "Controller Object Reference"))
  (returns (ReturnValue :type "Object Class Reference"))
  (bind _asps_arena (cast `/Game/_Source/Arena/PS_Arena` (`Controller.PlayerState` InController)))
  (return (`/Game/_Source/Arena/PS_Arena.CharacterClass` _asps_arena)))

(fn `UserConstructionScript`)